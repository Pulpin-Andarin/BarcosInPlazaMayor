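; BP_ShipAIController is an AI controller for ships that targets the player's pawn.
; On possess, it runs its assigned behavior tree, then seeds the Blackboard with the first player pawn as target, plus the attack radius and wait time.
; Key names and tuning values come from variables, and all further decision logic is left to the behavior tree.
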(event `self.ReceivePossess`
  (params (PossessedPawn :type "Pawn Object Reference"))
  (`self.RunBehaviorTree` (`self.BehaviorTree`))
  (`BlackboardComponent.SetValueAsObject` (`self.Blackboard`) (`self.TargetName`) (`GameplayStatics.GetPlayerPawn` 0))
  (`BlackboardComponent.SetValueAsFloat` (`self.Blackboard`) (`self.AttackRadiusName`) (`self.AttackRadius`))
  (`BlackboardComponent.SetValueAsFloat` (`self.Blackboard`) (`self.WaitTimeName`) (`self.WaitTime`)))

(fn `UserConstructionScript`)