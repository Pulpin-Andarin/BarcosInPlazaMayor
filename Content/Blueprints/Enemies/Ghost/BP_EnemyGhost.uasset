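; BP_EnemyGhost is a ghost enemy boat that damages the player's boat on contact.
; On BeginPlay it starts the ability in its BPGhostComponent.
; Root overlap with the player pawn casts it to BP_Boat and applies damage through its Health component.
; A separate Ghost function attaches smoke to Root and loops over BoatMesh's material slots to swap in a new material.
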(event `self.ReceiveBeginPlay`
  (`/Game/Blueprints/Enemies/Ghost/BP_GhostComponent.Ghost Ability` (`self.BP_GhostComponent1`)))

(event `self.Root.OnComponentBeginOverlap`
  (params (OverlappedComponent :type "PrimitiveComponent Object Reference") (OtherActor :type "Actor Object Reference") (OtherComp :type "PrimitiveComponent Object Reference") (OtherBodyIndex :type Integer) (bFromSweep :type Boolean) (SweepResult :type "HitResult Structure (by ref)"))
  (if (== OtherActor (`GameplayStatics.GetPlayerPawn` 0))
    (bind _asbp_boat (cast `/Game/Blueprints/Ship/BP_Boat` OtherActor))
    (bind _health (`/Game/Blueprints/Ship/BP_Boat.Health` _asbp_boat))
    (`HealthComponent.Damage` _health (`self.Damage_0`))
    (bind _returnvalue (`HealthComponent.GetCurrentHealth` _health))))

(event `self.ReceiveTick`
  (params (DeltaSeconds :type "Float (single-precision)")))

(fn `Ghost`
  (bind _cont_0 (`self.Cont_0`))
  (`GameplayStatics.SpawnEmitterAttached` "/Game/Realistic_Starter_VFX_Pack_Vol2/Particles/Smoke/P_Smoke_F.P_Smoke_F" (`self.Root`))
  (if (< _cont_0 18.0) :!label _label
    (`PrimitiveComponent.SetMaterial` (`self.BoatMesh`) (`KismetMathLibrary.Conv_Int64ToInt` (`KismetMathLibrary.Conv_DoubleToInt64` _cont_0)) "/Game/Blueprints/Enemies/Ghost/NewMaterial.NewMaterial")
    (set `self.Cont_0` (+ (`self.Cont_0`) 1.0))
    (goto _label)))

(fn `UserConstructionScript`
  (`parent.UserConstructionScript`))