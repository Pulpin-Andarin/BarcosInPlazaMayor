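; BP_EnemyGhostChild is a ghost enemy that damages the player's boat on contact.
; On BeginPlay it triggers GhostAbility on its BPGhostComponent, then runs the parent's BeginPlay.
; When the Root component overlaps the player pawn, it casts to BP_Boat and applies its Damage value through the boat's Health component.
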(event `self.Root.OnComponentBeginOverlap`
  (params (OverlappedComponent :type "PrimitiveComponent Object Reference") (OtherActor :type "Actor Object Reference") (OtherComp :type "PrimitiveComponent Object Reference") (OtherBodyIndex :type Integer) (bFromSweep :type Boolean) (SweepResult :type "HitResult Structure (by ref)"))
  (if (== OtherActor (`GameplayStatics.GetPlayerPawn` 0))
    (bind _asbp_boat (cast `/Game/Blueprints/Ship/BP_Boat` OtherActor))
    (bind _health (`/Game/Blueprints/Ship/BP_Boat.Health` _asbp_boat))
    (`HealthComponent.Damage` _health (`self.Damage`))
    (bind _returnvalue (`HealthComponent.GetCurrentHealth` _health))))

(event `self.ReceiveBeginPlay`
  (`/Game/Blueprints/Enemies/Ghost/BP_GhostComponent.Ghost Ability` (`self.BP_GhostComponent`))
  (`parent.ReceiveBeginPlay`))

(fn `UserConstructionScript`
  (`parent.UserConstructionScript`))