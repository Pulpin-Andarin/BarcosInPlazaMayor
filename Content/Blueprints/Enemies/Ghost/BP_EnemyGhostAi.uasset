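; BP_EnemyGhostAi is a ghost enemy that damages the player's boat on contact.
; On BeginPlay it triggers the ghost component's ability, runs parent setup, deactivates the inherited follow camera and caches its life bar widget.
; Root overlaps with the player pawn apply damage through BP_Boat's Health component.
; Its own Health update event refreshes the life bar, while movement and AI logic are absent from this graph.
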(event `self.Root.OnComponentBeginOverlap`
  (params (OverlappedComponent :type "PrimitiveComponent Object Reference") (OtherActor :type "Actor Object Reference") (OtherComp :type "PrimitiveComponent Object Reference") (OtherBodyIndex :type Integer) (bFromSweep :type Boolean) (SweepResult :type "HitResult Structure (by ref)"))
  (if (== OtherActor (`GameplayStatics.GetPlayerPawn` 0))
    (bind _asbp_boat (cast `/Game/Blueprints/Ship/BP_Boat` OtherActor))
    (bind _health (`/Game/Blueprints/Ship/BP_Boat.Health` _asbp_boat))
    (`HealthComponent.Damage` _health (`self.Damage`))
    (bind _returnvalue (`HealthComponent.GetCurrentHealth` _health))))

(event `self.ReceiveBeginPlay`
  (`/Game/Blueprints/Enemies/Ghost/BP_GhostComponent.Ghost Ability` (`self.BP_GhostComponent`))
  (`parent.ReceiveBeginPlay`)
  (`ActorComponent.Deactivate` (`self.FollowCamera`))
  (bind _asw_enemy_life_bar (cast `/Game/UI/W_EnemyLifeBar` (`WidgetComponent.GetUserWidgetObject` (`self.LifeBar`))))
  (set `self.W Enemy Life Bar` _asw_enemy_life_bar))

(event `self.ReceiveTick`
  (params (DeltaSeconds :type "Float (single-precision)"))
  (`parent.ReceiveTick` DeltaSeconds))

(event `self.Health.UpdateLifeEvent`
  (bind _w_enemy_life_bar (`self.W Enemy Life Bar`))
  (bind _health (`self.Health`))
  (bind _returnvalue (`HealthComponent.GetMaxHealth` _health))
  (bind _returnvalue_2 (`HealthComponent.GetCurrentHealth` _health))
  (`/Engine/EditorBlueprintResources/StandardMacros.IsValid` _w_enemy_life_bar
    (:`Is Valid`
      (`/Game/UI/W_EnemyLifeBar.UpdateLifeBar` _w_enemy_life_bar _returnvalue _returnvalue_2))))

(fn `UserConstructionScript`
  (`parent.UserConstructionScript`))