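; BP_ShipAIControllerGhost is the AI controller for the Ghost ship enemy.
; On BeginPlay it initializes the BB_ShipGhost blackboard and runs the assigned behavior tree.
; It then seeds the blackboard with the first player pawn as the target, along with its attack radius and reload time, using key names held in variables.
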(event `self.ReceiveBeginPlay`
  (bind _blackboardcomponent (`self.UseBlackboard` "/Game/Blueprints/Enemies/Ghost/AI/BB_ShipGhost.BB_ShipGhost"))
  (set `self.BlackboardData` _blackboardcomponent)
  (`self.RunBehaviorTree` (`self.BehaviorTree`))
  (`BlackboardComponent.SetValueAsObject` (`self.BlackboardData`) (`self.TargetName`) (`GameplayStatics.GetPlayerPawn` 0))
  (`BlackboardComponent.SetValueAsFloat` (`self.BlackboardData`) (`self.AttackRadiusName`) (`self.AttackRadius`))
  (`BlackboardComponent.SetValueAsFloat` (`self.BlackboardData`) (`self.ReloadTimeName`) (`self.ReloadTime`)))

(fn `UserConstructionScript`)