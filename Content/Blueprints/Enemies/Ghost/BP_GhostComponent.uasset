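; BP_GhostComponent is an enemy component that gives its owning Boat a ghost look when GhostAbility fires.
; The Ghost function attaches a smoke emitter to the boat's root, then loops a float counter to apply NewMaterial to the first 18 material slots of BoatMesh.
; The counter is never reset within the graphs, and DamageGhost is an empty stub.
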(event `Ghost Ability`
  (`self.Ghost` (`self.GetOwner`)))

(event `Damage Ghost`)

(fn `Ghost`
  (params (Owner :type "Actor Object Reference"))
  (bind _cont (`self.Cont`))
  (bind _asboat (cast `Boat` Owner))
  (`GameplayStatics.SpawnEmitterAttached` "/Game/Realistic_Starter_VFX_Pack_Vol2/Particles/Smoke/P_Smoke_F.P_Smoke_F" (`Boat.Root` _asboat))
  (if (< _cont 18.0) :!label _label
    (`PrimitiveComponent.SetMaterial` (`Boat.BoatMesh` _asboat) (`KismetMathLibrary.Conv_Int64ToInt` (`KismetMathLibrary.Conv_DoubleToInt64` _cont)) "/Game/Blueprints/Enemies/Ghost/NewMaterial.NewMaterial")
    (set `self.Cont` (+ _cont 1.0))
    (goto _label)))