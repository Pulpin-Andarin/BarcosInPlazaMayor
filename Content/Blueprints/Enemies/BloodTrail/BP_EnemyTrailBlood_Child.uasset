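; Enemy blood trail Blueprint, a child class whose Niagara particles damage the player boat.
; On BeginPlay it deactivates the follow camera and registers itself as the Niagara export callback through User.BPCallback.
; When particle data arrives and BloodTrailAbility is ready, it sphere-traces at each particle position, ignoring itself.
; Each BP_Boat hit takes the ability's damage and starts its cooldown, which is checked only once per batch.
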(event `self.ReceiveBeginPlay`
  (`parent.ReceiveBeginPlay`)
  (`ActorComponent.Deactivate` (`self.FollowCamera`))
  (`NiagaraComponent.SetNiagaraVariableObject` (`self.NS_TrailBlood`) "User.BPCallback" self)
  (`KismetArrayLibrary.Array_Add` (`self.Actors to Ignore`) self))

(event `self.ReceiveParticleData`
  (params (Data :type "Array of BasicParticleData Structure (by ref)") (NiagaraSystem :type "NiagaraSystem Object Reference") (SimulationPositionOffset :type "Vector Structure (by ref)"))
  (if (`BloodTrailAbility.bCanExecuteAbility` (`self.BloodTrailAbility`))
    (for _array_element Data
      (bind _outhit (`KismetSystemLibrary.SphereTraceSingleForObjects` (`.Position` (break `BasicParticleData` _array_element)) (0.0 0.0 0.0) 100.0 (`self.Object Types_0`) false (`self.Actors to Ignore`)))
      (bind _asbp_boat (cast `/Game/Blueprints/Ship/BP_Boat` (`.HitActor` (`GameplayStatics.BreakHitResult` _outhit))))
      (`HealthComponent.Damage` (`/Game/Blueprints/Ship/BP_Boat.Health` _asbp_boat) (`BloodTrailAbility.Damage` (`self.BloodTrailAbility`)))
      (`BloodTrailAbility.ActivateCooldown` (`self.BloodTrailAbility`)))))

(fn `UserConstructionScript`
  (`parent.UserConstructionScript`))