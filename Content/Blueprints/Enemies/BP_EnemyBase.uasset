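; Base enemy Blueprint that manages an on-screen life bar and death handling for a pawn with a Health component and floating movement.
; At BeginPlay it deactivates the inherited follow camera and caches the LifeBar widget, which Health update events refresh with current and maximum health.
; On death it overrides the root's mass, stops movement and destroys the actor after a delay.
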(event `self.Health.Dead`
  (`PrimitiveComponent.SetMassOverrideInKg` (`self.Root`) "None" 350.0 true)
  (`ActorComponent.Deactivate` (`self.FloatingPawnMovement`))
  (`KismetSystemLibrary.Delay` 7.0)
  (`self.K2_DestroyActor`))

(event `self.ReceiveBeginPlay`
  (`parent.ReceiveBeginPlay`)
  (`ActorComponent.Deactivate` (`self.FollowCamera`))
  (bind _asw_enemy_life_bar (cast `/Game/UI/W_EnemyLifeBar` (`WidgetComponent.GetUserWidgetObject` (`self.LifeBar`))))
  (set `self.W Enemy Life Bar` _asw_enemy_life_bar))

(event `self.ReceiveTick`
  (params (DeltaSeconds :type "Float (single-precision)"))
  (`parent.ReceiveTick` DeltaSeconds))

(event `self.Health.UpdateLifeEvent`
  (bind _w_enemy_life_bar (`self.W Enemy Life Bar`))
  (bind _health (`self.Health`))
  (bind _returnvalue (`HealthComponent.GetMaxHealth` _health))
  (bind _returnvalue_2 (`HealthComponent.GetCurrentHealth` _health))
  (`/Engine/EditorBlueprintResources/StandardMacros.IsValid` _w_enemy_life_bar
    (:`Is Valid`
      (`/Game/UI/W_EnemyLifeBar.UpdateLifeBar` _w_enemy_life_bar _returnvalue _returnvalue_2))))

(fn `UserConstructionScript`
  (`parent.UserConstructionScript`))