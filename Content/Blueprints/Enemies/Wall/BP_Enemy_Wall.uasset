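; BP_Enemy_Wall is an enemy Blueprint with a timed, Niagara-driven wall ability.
; BeginPlay passes the ability duration and itself as callback object to the Niagara system, adds itself to BPWallComponent's ignore list, and starts the effect inactive.
; When the component allows it, UseHability activates the effect, then chained timers deactivate it after the duration and re-enable the ability after the cooldown.
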(event `self.ReceiveBeginPlay`
  (`parent.ReceiveBeginPlay`)
  (`FXSystemComponent.SetFloatParameter` (`self.NS_Wall`) "DurationHability" (`/Game/Blueprints/Enemies/Wall/BP_WallComponent.HabilityDuration` (`self.BP_WallComponent`)))
  (`NiagaraComponent.SetNiagaraVariableObject` (`self.NS_Wall`) "User.BPCallBack" self)
  (`KismetArrayLibrary.Array_Add` (`/Game/Blueprints/Enemies/Wall/BP_WallComponent.ActorsToIgnore` (`self.BP_WallComponent`)) self)
  (`ActorComponent.SetActive` (`self.NS_Wall`) false false))

(event `UseHability`
  (if (`/Game/Blueprints/Enemies/Wall/BP_WallComponent.CanUseHability` (`self.BP_WallComponent`))
    (`ActorComponent.SetActive` (`self.NS_Wall`) true false)
    (set `/Game/Blueprints/Enemies/Wall/BP_WallComponent.CanUseHability` false (`self.BP_WallComponent`))
    (`KismetSystemLibrary.K2_SetTimer` null "DeactivateHability" (`/Game/Blueprints/Enemies/Wall/BP_WallComponent.HabilityDuration` (`self.BP_WallComponent`)))))

(fn `ActivateHability`
  (set `/Game/Blueprints/Enemies/Wall/BP_WallComponent.CanUseHability` true (`self.BP_WallComponent`)))

(fn `DeactivateHability`
  (`ActorComponent.SetActive` (`self.NS_Wall`) false false)
  (`KismetSystemLibrary.K2_SetTimer` null "ActivateHability" (`/Game/Blueprints/Enemies/Wall/BP_WallComponent.CooldownHability` (`self.BP_WallComponent`))))

(fn `UserConstructionScript`
  (`parent.UserConstructionScript`))