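; AI controller for the Wall enemy ship, which sets up its behavior tree and blackboard.
; On BeginPlay it initializes the BB_Ship_Wall blackboard and runs the assigned behavior tree.
; It then seeds the blackboard once with the first player's pawn as target, plus its own attack radius and reload time.
; It has no Tick or other runtime logic of its own.
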(event `self.ReceiveBeginPlay`
  (bind _blackboardcomponent (`self.UseBlackboard` "/Game/Blueprints/Enemies/Wall/AI/BB_Ship_Wall.BB_Ship_Wall"))
  (set `self.BlackboardData` _blackboardcomponent)
  (`self.RunBehaviorTree` (`self.BehaviorTree`))
  (`BlackboardComponent.SetValueAsObject` (`self.BlackboardData`) (`self.TargetName`) (`GameplayStatics.GetPlayerPawn` 0))
  (`BlackboardComponent.SetValueAsFloat` (`self.BlackboardData`) (`self.AttackRadiusName`) (`self.AttackRadius`))
  (`BlackboardComponent.SetValueAsFloat` (`self.BlackboardData`) (`self.ReloadTimeName`) (`self.ReloadTime`)))

(fn `UserConstructionScript`)