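; Wall enemy component that damages boats touched by its Niagara particles.
; An event receives exported Niagara particle data and runs a sphere trace at each particle position.
; A hit BP_Boat takes damage through its Health and joins the trace's ignore list, so later traces skip it and it is not damaged again.
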(event `CustomEvent`
  (params (Data :type "Array of BasicParticleData Structure (by ref)") (NiagaraSystem :type "NiagaraSystem Object Reference") (SimulationPositionOffset :type "Vector Structure (by ref)"))
  (for _array_element Data
    (bind _outhit (`KismetSystemLibrary.SphereTraceSingleForObjects` (`.Position` (break `BasicParticleData` _array_element)) (0.0 0.0 0.0) 100.0 (`self.ObjectTypes`) false (`self.ActorsToIgnore`)))
    (bind _asbp_boat (cast `/Game/Blueprints/Ship/BP_Boat` (`.HitActor` (`GameplayStatics.BreakHitResult` _outhit))))
    (`HealthComponent.Damage` (`/Game/Blueprints/Ship/BP_Boat.Health` _asbp_boat) (`self.Damage`))
    (`KismetArrayLibrary.Array_Add` (`self.ActorsToIgnore`) (`.HitActor` (`GameplayStatics.BreakHitResult` _outhit)))))