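; Actor component that gives a Boat owner a timed forward charge, stored under enemy assets.
; ChargeAbility caches the boat and its max speed, raises that limit and starts the countdown, ignoring calls while already charging.
; Tick sets floating-movement acceleration and pushes the boat along its forward vector until time runs out.
; On expiry it restores the saved max speed but leaves acceleration changed.
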(event `self.ReceiveBeginPlay`)

(event `self.ReceiveTick`
  (params (DeltaSeconds :type "Float (single-precision)"))
  (bind _boat_ref (`self.Boat Ref`))
  (if (`self.Charging`)
    (`/Engine/EditorBlueprintResources/StandardMacros.IsValid` (`self.Boat Ref`)
      (:`Is Valid`
        (bind _output_get (set `FloatingPawnMovement.Acceleration` (`self.AccelerationRate`) (`Boat.FloatingMovementComponent` _boat_ref)))
        (`Pawn.AddMovementInput` _boat_ref (`Actor.GetActorForwardVector` (`self.GetOwner`)) _output_get false)
        (bind _output_get_2 (set `self.RemainingChargeDuration` (- (`self.RemainingChargeDuration`) DeltaSeconds)))
        (if (<= _output_get_2 0.0)
          (set `self.Charging` false)
          (set `FloatingPawnMovement.MaxSpeed` (`self.InitialMaxSpeed`) (`Boat.FloatingMovementComponent` (`self.Boat Ref`))))))))

(event `ChargeAbility`
  (if (not (`self.Charging`))
    (set `self.RemainingChargeDuration` (`self.ChargeDuration`))
    (bind _asboat (cast `Boat` (`self.GetOwner`)))
    (`/Engine/EditorBlueprintResources/StandardMacros.IsValid` _asboat
      (:`Is Valid`
        (set `self.Boat Ref` _asboat)
        (bind _floatingmovementcomponent (`Boat.FloatingMovementComponent` _asboat))
        (set `self.InitialMaxSpeed` (`FloatingPawnMovement.MaxSpeed` _floatingmovementcomponent))
        (set `FloatingPawnMovement.MaxSpeed` (`self.MaxSpeed`) _floatingmovementcomponent)
        (set `self.Charging` true)
        (set `self.RemainingChargeDuration` (`self.ChargeDuration`))))))