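; Rhino variant of the player boat, with a charge attack that damages boats it rams.
; Pressing Space Bar triggers the ability on its BPChargeComponent.
; While that component is charging, any BP_Boat that begins overlapping this boat takes ChargeDamage through its Health.
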(event `self.ReceiveActorBeginOverlap`
  (params (OtherActor :type "Actor Object Reference"))
  (if (`/Game/Blueprints/Enemies/Charge/BP_ChargeComponent.Charging` (`self.BP_ChargeComponent`))
    (bind _asbp_boat (cast `/Game/Blueprints/Ship/BP_Boat` OtherActor))
    (`HealthComponent.Damage` (`/Game/Blueprints/Ship/BP_Boat.Health` _asbp_boat) (`self.ChargeDamage`))))

(event `Key|SpaceBar`
  (params (Key :type "Key Structure"))
  (:`Pressed`
    (`/Game/Blueprints/Enemies/Charge/BP_ChargeComponent.ChargeAbility` (`self.BP_ChargeComponent`))))

(fn `UserConstructionScript`
  (`parent.UserConstructionScript`))