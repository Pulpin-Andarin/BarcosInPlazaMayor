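; Player boat with left and right broadside cannons and a ghost ability that damages other BP_Boat actors on overlap.
; Holding fire runs a looping timer that builds launch impulse and redraws the predicted arc with spline meshes and a target decal that flags boats.
; Release fires through BoatShootComponent and starts that side's reload, driving VFX and HUD.
; Health hits trigger chained timelines that roll the mesh, while rotation events update the HUD.
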(event `self.Health.HittedEvent`
  (bind _boatmesh (`self.BoatMesh`))
  (bind _boatmesh_2 (`self.BoatMesh`))
  (bind _boatmesh_3 (`self.BoatMesh`))
  (bind (_relativerotation_roll _relativerotation_pitch _relativerotation_yaw) (`KismetMathLibrary.BreakRotator` (`SceneComponent.RelativeRotation` _boatmesh)))
  (bind (_relativerotation_roll_2 _relativerotation_pitch_2 _relativerotation_yaw_2) (`KismetMathLibrary.BreakRotator` (`SceneComponent.RelativeRotation` _boatmesh_2)))
  (bind (_relativerotation_roll_3 _relativerotation_pitch_3 _relativerotation_yaw_3) (`KismetMathLibrary.BreakRotator` (`SceneComponent.RelativeRotation` _boatmesh_3)))
  (`/Engine/EditorBlueprintResources/StandardMacros.DoOnce` false :!label _label
    (:`Completed`
      (`KismetSystemLibrary.PrintString` "Hit")
      (bind (_direction _boat_hitted) (`Timeline|Timeline` :!via `PlayFromStart`)
        (:`Update`
          (bind _returnvalue (`KismetMathLibrary.Lerp` 0.0 0.1 _boat_hitted))
          (`SceneComponent.K2_SetRelativeRotation` _boatmesh (`KismetMathLibrary.MakeRotator` (+ _relativerotation_roll _returnvalue) _relativerotation_pitch _relativerotation_yaw) false false))
        (:`Finished`
          (bind (_direction_2 _boat_hitted_2) (`Timeline|Timeline_0` :!via `PlayFromStart`)
            (:`Update`
              (bind _returnvalue_2 (+ _relativerotation_roll_2 (`KismetMathLibrary.Lerp` 0.0 -0.2 _boat_hitted_2)))
              (`SceneComponent.K2_SetRelativeRotation` _boatmesh_2 (`KismetMathLibrary.MakeRotator` _returnvalue_2 _relativerotation_pitch_2 _relativerotation_yaw_2) false false))
            (:`Finished`
              (bind (_direction_3 _boat_hitted_3) (`Timeline|Timeline_1` :!via `PlayFromStart`)
                (:`Update`
                  (`SceneComponent.K2_SetRelativeRotation` _boatmesh_3 (`KismetMathLibrary.MakeRotator` (`KismetMathLibrary.Lerp` (+ (- _returnvalue 0.0) (+ _returnvalue_2 0.0)) 90.0 _boat_hitted_3) _relativerotation_pitch_3 _relativerotation_yaw_3) false false))
                (:`Finished`
                  (goto _label :!via `Reset`))))))))))

(event `self.Root.OnComponentBeginOverlap`
  (params (OverlappedComponent :type "PrimitiveComponent Object Reference") (OtherActor :type "Actor Object Reference") (OtherComp :type "PrimitiveComponent Object Reference") (OtherBodyIndex :type Integer) (bFromSweep :type Boolean) (SweepResult :type "HitResult Structure (by ref)"))
  (if (`/Game/Blueprints/Enemies/Ghost/BP_GhostComponent.GhostTime` (`self.BP_GhostComponent`))
    (if (!= OtherActor self)
      (bind _asbp_boat (cast `/Game/Blueprints/Ship/BP_Boat` OtherActor))
      (`HealthComponent.Damage` (`/Game/Blueprints/Ship/BP_Boat.Health` _asbp_boat) (`self.GhostDamage`)))))

(event `Key|ñ`
  (params (Key :type "Key Structure"))
  (bind _bp_ghostcomponent (`self.BP_GhostComponent`))
  (:`Pressed`
    (set `/Game/Blueprints/Enemies/Ghost/BP_GhostComponent.GhostTime` true _bp_ghostcomponent)
    (`/Game/Blueprints/Enemies/Ghost/BP_GhostComponent.Ghost Ability` _bp_ghostcomponent)))

(event `self.ReceiveBeginPlay`
  (bind _returnvalue (`GameplayStatics.GetPlayerCameraManager` 0))
  (add `self.RotateBoatEvent` (delegate `RotateBoatEvent_Event`))
  (set `PlayerCameraManager.ViewPitchMin` -70.0 _returnvalue)
  (set `PlayerCameraManager.ViewPitchMax` 45.0 _returnvalue))

(event `RotateBoatEvent_Event` :!signature `self.RotateBoatEvent`
  (params (direccion :type Boolean))
  (bind _asbp_hud (cast `/Game/Blueprints/HUD/BP_Hud` (`PlayerController.GetHUD` (`GameplayStatics.GetPlayerController` 0))))
  (bind _hudreference (`/Game/Blueprints/HUD/BP_Hud.HudReference` _asbp_hud))
  (`/Engine/EditorBlueprintResources/StandardMacros.IsValid` _hudreference
    (:`Is Valid`
      (`/Game/UI/W_GameplayUIBlueprint.Rotating` _hudreference direccion))))

(event `self.ReceiveTick`
  (params (DeltaSeconds :type "Float (single-precision)")))

(event `EnhancedInput|/Game/ThirdPerson/Input/Actions/IA_ShootRight`
  (params (ActionValue :type Boolean) (ElapsedSeconds :type "Float (double-precision)") (TriggeredSeconds :type "Float (double-precision)") (InputAction :type "InputAction Object Reference" :default "/Game/ThirdPerson/Input/Actions/IA_ShootRight.IA_ShootRight"))
  (bind _boatshootcomponent (`self.BoatShootComponent`))
  (:`Started`
    (if (`BoatShootComponent.bReloadingRight` _boatshootcomponent)
      _
      (elif (not (`BoatShootComponent.bAiming` _boatshootcomponent))
        (bind _returnvalue (`KismetSystemLibrary.K2_SetTimerDelegate` (delegate `ShootRight`) 0.1 true))
        (set `self.RightTimerHandler` _returnvalue)
        (`self.InitValuesForPrediction`)
        (set `self.AimingRight` true))))
  (:`Completed`
    (if (`self.AimingRight`)
      (`BoatShootComponent.StartReloadingRightSide` (`self.BoatShootComponent`))
      (`self.ShootAndClearTimersInDirection` (`self.RightArrow`) (`self.RightTimerHandler`))
      (set `self.AimingRight` false))))

(event `ShootRight`
  (`self.ShowShootPrediction` (`self.RightArrow`)))

(event `EnhancedInput|/Game/ThirdPerson/Input/Actions/IA_ShootLeft`
  (params (ActionValue :type Boolean) (ElapsedSeconds :type "Float (double-precision)") (TriggeredSeconds :type "Float (double-precision)") (InputAction :type "InputAction Object Reference" :default "/Game/ThirdPerson/Input/Actions/IA_ShootLeft.IA_ShootLeft"))
  (:`Started`
    (if (`BoatShootComponent.bReloadingLeft` (`self.BoatShootComponent`))
      _
      (elif (not (`BoatShootComponent.bAiming` (`self.BoatShootComponent`)))
        (bind _returnvalue (`KismetSystemLibrary.K2_SetTimerDelegate` (delegate `ShootLeft`) 0.1 true))
        (set `self.LeftTimerHandler` _returnvalue)
        (`self.InitValuesForPrediction`)
        (set `self.AimingLeft` true))))
  (:`Completed`
    (if (`self.AimingLeft`)
      (`self.ShootAndClearTimersInDirection` (`self.LeftArrow`) (`self.LeftTimerHandler`))
      (set `self.AimingLeft` false)
      (`BoatShootComponent.StartReloadingLeftSide` (`self.BoatShootComponent`)))))

(event `ShootLeft`
  (`self.ShowShootPrediction` (`self.LeftArrow`)))

(event `self.BoatShootComponent.EndVfxRight`
  ;[1 1 1] VFX recharge
  (`ActorComponent.Deactivate` (`self.RightShoot`)))

(event `self.BoatShootComponent.EndVfxLeft`
  ;[1 1 1] VFX recharge
  (`ActorComponent.Deactivate` (`self.LeftShoot`)))

(event `self.BoatShootComponent.StartVfxRight`
  ;[1 1 1] VFX recharge
  (`ActorComponent.Activate` (`self.RightShoot`) false)
  (bind _asbp_hud (cast `/Game/Blueprints/HUD/BP_Hud` (`PlayerController.GetHUD` (`GameplayStatics.GetPlayerController` 0))))
  (bind _hudreference (`/Game/Blueprints/HUD/BP_Hud.HudReference` _asbp_hud))
  (`/Engine/EditorBlueprintResources/StandardMacros.IsValid` _hudreference
    (:`Is Valid`
      (`/Game/UI/W_GameplayUIBlueprint.CanonRightStart` _hudreference (`BoatShootComponent.RightReloadingTime` (`self.BoatShootComponent`))))))

(event `self.BoatShootComponent.StartVfxLeft`
  ;[1 1 1] VFX recharge
  (`ActorComponent.Activate` (`self.LeftShoot`) false)
  (bind _asbp_hud (cast `/Game/Blueprints/HUD/BP_Hud` (`PlayerController.GetHUD` (`GameplayStatics.GetPlayerController` 0))))
  (bind _hudreference (`/Game/Blueprints/HUD/BP_Hud.HudReference` _asbp_hud))
  (`/Engine/EditorBlueprintResources/StandardMacros.IsValid` _hudreference
    (:`Is Valid`
      (`/Game/UI/W_GameplayUIBlueprint.CanonLeftStart` _hudreference (`BoatShootComponent.LeftReloadingTime` (`self.BoatShootComponent`))))))

(fn `clear arc`
  (bind _spline_meshes (`self.Spline Meshes`))
  (`ActorComponent.K2_DestroyComponent` _spline_meshes)
  (`KismetArrayLibrary.Array_Clear` _spline_meshes)
  (`SplineComponent.ClearSplinePoints` (`self.Spline`) true))

(fn `InitValuesForPrediction`
  (bind _boatshootcomponent (`self.BoatShootComponent`))
  (`SceneComponent.SetVisibility` (`self.Sphere`) true false)
  (`SceneComponent.SetVisibility` (`self.DecalShootTarget`) true false)
  (set `BoatShootComponent.ActualImpulse` (`BoatShootComponent.MinImpulse` _boatshootcomponent) _boatshootcomponent)
  (set `BoatShootComponent.bAiming` true (`self.BoatShootComponent`)))

(fn `InitValuesForPrediction_0`
  (bind _boatshootcomponent (`self.BoatShootComponent`))
  (`SceneComponent.SetVisibility` (`self.DecalShootTarget`) true false)
  (set `BoatShootComponent.ActualImpulse` (`BoatShootComponent.MinImpulse` _boatshootcomponent) _boatshootcomponent)
  (set `BoatShootComponent.bAiming` true (`self.BoatShootComponent`)))

(fn `SetActualImpulse`
  (returns (ActualImpulse :type "Float (single-precision)"))
  (bind _boatshootcomponent (`self.BoatShootComponent`))
  (bind _actualimpulse (`BoatShootComponent.ActualImpulse` _boatshootcomponent))
  (set `BoatShootComponent.ActualImpulse` (`KismetMathLibrary.FClamp` (+ _actualimpulse (`BoatShootComponent.ImpulsIncrement` _boatshootcomponent)) (`BoatShootComponent.MinImpulse` _boatshootcomponent) (`BoatShootComponent.MaxImpulse` _boatshootcomponent)) _boatshootcomponent)
  (return _actualimpulse))

(fn `ShootAndClearTimersInDirection`
  (params (Arrow :type "ArrowComponent Object Reference") (TimerHandler :type "TimerHandle Structure"))
  (bind _boatshootcomponent (`self.BoatShootComponent`))
  (bind _boatshootcomponent_2 (`self.BoatShootComponent`))
  (`BoatShootComponent.Shoot` _boatshootcomponent (`KismetMathLibrary.MakeTransform` (`SceneComponent.K2_GetComponentLocation` Arrow) (`SceneComponent.K2_GetComponentRotation` Arrow)) (`BoatShootComponent.ActualImpulse` _boatshootcomponent))
  (`self.clear arc`)
  (`KismetSystemLibrary.K2_ClearAndInvalidateTimerHandle` TimerHandler)
  (`SceneComponent.SetVisibility` (`self.DecalShootTarget`) false false)
  (set `BoatShootComponent.ActualImpulse` (`BoatShootComponent.MinImpulse` _boatshootcomponent_2) _boatshootcomponent_2)
  (set `BoatShootComponent.bAiming` false (`self.BoatShootComponent`))
  (`SceneComponent.SetVisibility` (`self.Sphere`) false false))

(fn `ShowShootPrediction`
  (params (Arrow :type "ArrowComponent Object Reference"))
  (bind _decalshoottarget (`self.DecalShootTarget`))
  (bind _spline (`self.Spline`))
  (bind _spline_2 (`self.Spline`))
  (bind _actualimpulse (`self.SetActualImpulse`))
  (bind _output_get (set `self.LastLaunchVelocity` (* (`SceneComponent.GetForwardVector` Arrow) _actualimpulse)))
  (`self.clear arc`)
  (bind _predictresult (`GameplayStatics.Blueprint_PredictProjectilePath_Advanced` (make `PredictProjectilePathParams` :`StartLocation` (`SceneComponent.K2_GetComponentLocation` Arrow) :`LaunchVelocity` _output_get :`bTraceWithCollision` true :`ProjectileRadius` 5.0 :`MaxSimTime` 5.0 :`ActorsToIgnore` (`|MakeArray` self :!type "Actor Object Reference"))))
  (bind (_bblockinghit _binitialoverlap _time _distance _location _impactpoint _normal _impactnormal _physmat _hitactor) (`GameplayStatics.BreakHitResult` (`.HitResult` (break `PredictProjectilePathResult` _predictresult))))
  (bind _returnvalue (`KismetMathLibrary.Conv_VectorToRotator` _normal))
  (`SceneComponent.K2_SetWorldLocationAndRotation` (`self.Sphere`) _location _returnvalue false false)
  (cast `/Game/Blueprints/Ship/BP_Boat` _hitactor
    (:`then`
      (`DecalComponent.SetDecalMaterial` _decalshoottarget "/Game/Materials/M_ShootTargetFound.M_ShootTargetFound"))
    (:`CastFailed`
      (`DecalComponent.SetDecalMaterial` _decalshoottarget "/Game/Materials/M_ShootTargetr.M_ShootTargetr")))
  (`SceneComponent.K2_SetWorldLocationAndRotation` _decalshoottarget _location _returnvalue false false)
  (for _array_element (break `PredictProjectilePathResult` _predictresult)
    (`SplineComponent.AddSplinePoint` _spline (`.Location` (break `PredictProjectilePathPointData` _array_element)) "Local" true))
  (`SplineComponent.SetSplinePointType` _spline (`KismetArrayLibrary.Array_LastIndex` (break `PredictProjectilePathResult` _predictresult)) "CurveClamped" true)
  (for _index (range (`SplineComponent.GetNumberOfSplinePoints` (`self.Spline`)))
    (bind _returnvalue_2 (`AddComponent|NODE_AddSplineMeshComponent-1` :`bManualAttachment` true))
    (`KismetArrayLibrary.Array_Add` (`self.Spline Meshes`) _returnvalue_2)
    (bind (_location_2 _tangent) (`SplineComponent.GetLocationAndTangentAtSplinePoint` _spline_2 _index "Local"))
    (bind (_location_3 _tangent_2) (`SplineComponent.GetLocationAndTangentAtSplinePoint` _spline_2 (+ _index 1) "Local"))
    (`SplineMeshComponent.SetStartAndEnd` _returnvalue_2 _location_2 _tangent _location_3 _tangent_2 true)))

(fn `UserConstructionScript`)