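; BP_BoatProjectileSlow is a ship projectile meant to slow the boat it hits.
; Its sphere overlap ignores the owning gunner and calls SlowVelocity on any BP_Boat, though both percent and time are passed as zero.
; On a boat hit it hides the projectile component and uses the ActiveParticle helper to activate wood destruction and explosion smoke effects at that component's location, without destroying the actor.
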(event `self.SphereComponent.OnComponentBeginOverlap`
  (params (OverlappedComponent :type "PrimitiveComponent Object Reference") (OtherActor :type "Actor Object Reference") (OtherComp :type "PrimitiveComponent Object Reference") (OtherBodyIndex :type Integer) (bFromSweep :type Boolean) (SweepResult :type "HitResult Structure (by ref)"))
  (if (not (== OtherActor (`self.OwnerGunner`)))
    (bind _asbp_boat (cast `/Game/Blueprints/Ship/BP_Boat` OtherActor))
    (`Boat.SlowVelocity` _asbp_boat 0.0 0.0)
    (`SceneComponent.SetVisibility` (`self.SphereProjectileComponent`) false false)
    (`self.ActiveParticle` (`self.P_WoodDestruction`))
    (`self.ActiveParticle` (`self.P_Explosion_Smoke`))))

(fn `ActiveParticle`
  (params (NewParam :type "SceneComponent Object Reference"))
  (`ActorComponent.Activate` NewParam false)
  (`SceneComponent.K2_SetWorldLocation` NewParam (`SceneComponent.K2_GetComponentLocation` (`self.SphereProjectileComponent`)) false true))

(fn `UserConstructionScript`)