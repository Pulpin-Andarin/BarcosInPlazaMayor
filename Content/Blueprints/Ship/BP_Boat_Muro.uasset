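; Boat with a Niagara wall ability, triggered by Space, that damages other boats and enemies.
; The wall runs for a set duration, then timers switch it off and re-enable the ability after a cooldown.
; Niagara exports particle data back to the Blueprint, which sphere-traces at each particle position and damages the hit actor's Health.
; Hit actors join an ignore list that is never cleared, so later activations skip them too.
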(event `self.ReceiveBeginPlay`
  (`parent.ReceiveBeginPlay`)
  (`FXSystemComponent.SetFloatParameter` (`self.NS_Wall`) "DurationHability" (`self.HabilityDuration`))
  (`NiagaraComponent.SetNiagaraVariableObject` (`self.NS_Wall`) "User.BPCallBack" self)
  (`KismetArrayLibrary.Array_Add` (`self.ActorsToIgnore`) self)
  (`ActorComponent.SetActive` (`self.NS_Wall`) false false))

(event `Key|SpaceBar`
  (params (Key :type "Key Structure"))
  (:`Pressed`
    (if (`self.CanUseHability`)
      (set `self.IsHabilityActive` false)
      (`ActorComponent.SetActive` (`self.NS_Wall`) true false)
      (set `self.CanUseHability` false)
      (`KismetSystemLibrary.K2_SetTimer` null "DeactivateHability" (`self.HabilityDuration`)))))

(event `self.ReceiveParticleData`
  (params (Data :type "Array of BasicParticleData Structure (by ref)") (NiagaraSystem :type "NiagaraSystem Object Reference") (SimulationPositionOffset :type "Vector Structure (by ref)"))
  (bind _damage (`self.Damage`))
  (bind _actorstoignore (`self.ActorsToIgnore`))
  (for _array_element Data
    (bind _outhit (`KismetSystemLibrary.SphereTraceSingleForObjects` (`.Position` (break `BasicParticleData` _array_element)) (0.0 0.0 0.0) 100.0 (`self.ObjectTypes`) false (`self.ActorsToIgnore`)))
    (bind _asbp_boat (cast `/Game/Blueprints/Ship/BP_Boat` (`.HitActor` (`GameplayStatics.BreakHitResult` _outhit)))
      (:`then`
        (bind _health (`/Game/Blueprints/Ship/BP_Boat.Health` _asbp_boat))
        (`HealthComponent.Damage` _health _damage)
        (`KismetArrayLibrary.Array_Add` _actorstoignore (`.HitActor` (`GameplayStatics.BreakHitResult` _outhit)))
        (`KismetSystemLibrary.PrintString` (`KismetStringLibrary.Conv_IntToString` (`HealthComponent.CurrentHealth` _health))))
      (:`CastFailed`
        (bind _asbp_enemy_base (cast `/Game/Blueprints/Enemies/BP_EnemyBase` (`.HitActor` (`GameplayStatics.BreakHitResult` _outhit))))
        (bind _health_2 (`/Game/Blueprints/Ship/BP_Boat.Health` _asbp_enemy_base))
        (`HealthComponent.Damage` _health_2 _damage)
        (`KismetArrayLibrary.Array_Add` _actorstoignore (`.HitActor` (`GameplayStatics.BreakHitResult` _outhit)))
        (`KismetSystemLibrary.PrintString` (`KismetStringLibrary.Conv_IntToString` (`HealthComponent.CurrentHealth` _health_2)))))))

(fn `ActivateHability`
  (set `self.CanUseHability` true))

(fn `DeactivateHability`
  (`ActorComponent.SetActive` (`self.NS_Wall`) false false)
  (`KismetSystemLibrary.K2_SetTimer` null "ActivateHability" (`self.CooldownHability`)))

(fn `UserConstructionScript`
  (`parent.UserConstructionScript`))