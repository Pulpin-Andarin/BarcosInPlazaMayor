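; Player 1's boat, which tilts its mesh on keyboard input and reports its health to the HUD.
; Timelines drive the mesh roll: holding A or D leans it to either side, and releasing eases it back toward upright.
; P triggers a chained hit wobble, gated by a DoOnce until it finishes.
; Health component events update the BP_Hud life display and print a debug message on death.
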(event `Key|D`
  (params (Key :type "Key Structure"))
  (bind _boatmesh (`self.BoatMesh`))
  (bind (_relativerotation_roll _relativerotation_pitch _relativerotation_yaw) (`KismetMathLibrary.BreakRotator` (`SceneComponent.RelativeRotation` _boatmesh)))
  (:`Pressed`
    (bind (_direction _boat_hitted) (`Timeline|Timeline_1_0` :!via `PlayFromStart`)
      (:`Update`
        (bind _returnvalue (`KismetMathLibrary.Lerp` 0.0 0.2 _boat_hitted))
        (`SceneComponent.K2_SetRelativeRotation` _boatmesh (`KismetMathLibrary.MakeRotator` (+ _relativerotation_roll _returnvalue) _relativerotation_pitch _relativerotation_yaw) false false))))
  (:`Released`
    (bind (_direction_2 _boat_hitted_2) (`Timeline|Timeline_3` :!via `PlayFromStart`)
      (:`Update`
        (`SceneComponent.K2_SetRelativeRotation` (`self.BoatMesh`) (`KismetMathLibrary.MakeRotator` (`KismetMathLibrary.Lerp` (- _relativerotation_roll _returnvalue) 90.0 _boat_hitted_2) 0.0 180.0) false false)))))

(event `Key|A`
  (params (Key :type "Key Structure"))
  (bind _boatmesh (`self.BoatMesh`))
  (bind (_relativerotation_roll _relativerotation_pitch _relativerotation_yaw) (`KismetMathLibrary.BreakRotator` (`SceneComponent.RelativeRotation` _boatmesh)))
  (:`Pressed`
    (bind (_direction _boat_hitted) (`Timeline|Timeline_4` :!via `PlayFromStart`)
      (:`Update`
        (bind _returnvalue (`KismetMathLibrary.Lerp` 0.0 -0.2 _boat_hitted))
        (`SceneComponent.K2_SetRelativeRotation` _boatmesh (`KismetMathLibrary.MakeRotator` (+ _relativerotation_roll _returnvalue) _relativerotation_pitch _relativerotation_yaw) false false))))
  (:`Released`
    (bind (_direction_2 _boat_hitted_2) (`Timeline|Timeline_5` :!via `PlayFromStart`)
      (:`Update`
        (`SceneComponent.K2_SetRelativeRotation` (`self.BoatMesh`) (`KismetMathLibrary.MakeRotator` (`KismetMathLibrary.Lerp` (- _relativerotation_roll _returnvalue) 90.0 _boat_hitted_2) 0.0 180.0) false false)))))

(event `Key|P`
  (params (Key :type "Key Structure"))
  (bind _boatmesh (`self.BoatMesh`))
  (bind _boatmesh_2 (`self.BoatMesh`))
  (bind _boatmesh_3 (`self.BoatMesh`))
  (bind (_relativerotation_roll _relativerotation_pitch _relativerotation_yaw) (`KismetMathLibrary.BreakRotator` (`SceneComponent.RelativeRotation` _boatmesh)))
  (bind (_relativerotation_roll_2 _relativerotation_pitch_2 _relativerotation_yaw_2) (`KismetMathLibrary.BreakRotator` (`SceneComponent.RelativeRotation` _boatmesh_2)))
  (bind (_relativerotation_roll_3 _relativerotation_pitch_3 _relativerotation_yaw_3) (`KismetMathLibrary.BreakRotator` (`SceneComponent.RelativeRotation` _boatmesh_3)))
  (:`Pressed`
    (`/Engine/EditorBlueprintResources/StandardMacros.DoOnce` false :!label _label
      (:`Completed`
        (`KismetSystemLibrary.PrintString` "Hit")
        (bind (_direction _boat_hitted) (`Timeline|Timeline_6` :!via `PlayFromStart`)
          (:`Update`
            (bind _returnvalue (`KismetMathLibrary.Lerp` 0.0 0.1 _boat_hitted))
            (`SceneComponent.K2_SetRelativeRotation` _boatmesh (`KismetMathLibrary.MakeRotator` (+ _relativerotation_roll _returnvalue) _relativerotation_pitch _relativerotation_yaw) false false))
          (:`Finished`
            (bind (_direction_2 _boat_hitted_2) (`Timeline|Timeline_0_0` :!via `PlayFromStart`)
              (:`Update`
                (bind _returnvalue_2 (+ _relativerotation_roll_2 (`KismetMathLibrary.Lerp` 0.0 -0.2 _boat_hitted_2)))
                (`SceneComponent.K2_SetRelativeRotation` _boatmesh_2 (`KismetMathLibrary.MakeRotator` _returnvalue_2 _relativerotation_pitch_2 _relativerotation_yaw_2) false false))
              (:`Finished`
                (bind (_direction_3 _boat_hitted_3) (`Timeline|Timeline_2` :!via `PlayFromStart`)
                  (:`Update`
                    (`SceneComponent.K2_SetRelativeRotation` _boatmesh_3 (`KismetMathLibrary.MakeRotator` (`KismetMathLibrary.Lerp` (+ (- _returnvalue 0.0) (+ _returnvalue_2 0.0)) 90.0 _boat_hitted_3) _relativerotation_pitch_3 _relativerotation_yaw_3) false false))
                  (:`Finished`
                    (goto _label :!via `Reset`)))))))))))

(event `self.ReceiveTick`
  (params (DeltaSeconds :type "Float (single-precision)"))
  (`parent.ReceiveTick` DeltaSeconds))

(event `self.Health.Dead`
  (`KismetSystemLibrary.PrintString` "Estas Muerto Perro"))

(event `self.Health.UpdateLifeEvent`
  (bind _health (`self.Health`))
  (bind _asbp_hud (cast `/Game/Blueprints/HUD/BP_Hud` (`PlayerController.GetHUD` (`GameplayStatics.GetPlayerController` 0))))
  (bind _hudreference (`/Game/Blueprints/HUD/BP_Hud.HudReference` _asbp_hud))
  (`/Engine/EditorBlueprintResources/StandardMacros.IsValid` _hudreference
    (:`Is Valid`
      (`/Game/UI/W_GameplayUIBlueprint.UpdateLife` _hudreference (`HealthComponent.CurrentHealth` _health) (`HealthComponent.MaxHealth` _health)))))

(fn `UserConstructionScript`
  (`parent.UserConstructionScript`))