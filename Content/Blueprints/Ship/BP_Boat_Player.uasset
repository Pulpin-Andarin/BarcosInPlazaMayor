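; Player boat Blueprint that handles steering tilt, health feedback, pausing and defeat.
; A and D presses drive timelines that roll the boat mesh sideways, and releases ease it back toward its resting rotation.
; BeginPlay shows the HUD and creates a hidden pause menu, revealed by IA_Pause, while Health events update the life display or open the Defeat level.
; GetAllGhostPoints returns the world locations of four ghost point components.
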(event `Key|D`
  (params (Key :type "Key Structure"))
  (bind _boatmesh (`self.BoatMesh`))
  (bind (_relativerotation_roll _relativerotation_pitch _relativerotation_yaw) (`KismetMathLibrary.BreakRotator` (`SceneComponent.RelativeRotation` _boatmesh)))
  (:`Pressed`
    (bind (_direction _boat_hitted) (`Timeline|Timeline_2` :!via `PlayFromStart`)
      (:`Update`
        (bind _returnvalue (`KismetMathLibrary.Lerp` 0.0 0.2 _boat_hitted))
        (`SceneComponent.K2_SetRelativeRotation` _boatmesh (`KismetMathLibrary.MakeRotator` (+ _relativerotation_roll _returnvalue) _relativerotation_pitch _relativerotation_yaw) false false))))
  (:`Released`
    (bind (_direction_2 _boat_hitted_2) (`Timeline|Timeline_3` :!via `PlayFromStart`)
      (:`Update`
        (`SceneComponent.K2_SetRelativeRotation` (`self.BoatMesh`) (`KismetMathLibrary.MakeRotator` (`KismetMathLibrary.Lerp` (- _relativerotation_roll _returnvalue) 90.0 _boat_hitted_2) 0.0 180.0) false false)))))

(event `Key|A`
  (params (Key :type "Key Structure"))
  (bind _boatmesh (`self.BoatMesh`))
  (bind (_relativerotation_roll _relativerotation_pitch _relativerotation_yaw) (`KismetMathLibrary.BreakRotator` (`SceneComponent.RelativeRotation` _boatmesh)))
  (:`Pressed`
    (bind (_direction _boat_hitted) (`Timeline|Timeline_4` :!via `PlayFromStart`)
      (:`Update`
        (bind _returnvalue (`KismetMathLibrary.Lerp` 0.0 -0.2 _boat_hitted))
        (`SceneComponent.K2_SetRelativeRotation` _boatmesh (`KismetMathLibrary.MakeRotator` (+ _relativerotation_roll _returnvalue) _relativerotation_pitch _relativerotation_yaw) false false))))
  (:`Released`
    (bind (_direction_2 _boat_hitted_2) (`Timeline|Timeline_5` :!via `PlayFromStart`)
      (:`Update`
        (`SceneComponent.K2_SetRelativeRotation` (`self.BoatMesh`) (`KismetMathLibrary.MakeRotator` (`KismetMathLibrary.Lerp` (- _relativerotation_roll _returnvalue) 90.0 _boat_hitted_2) 0.0 180.0) false false)))))

(event `self.ReceiveBeginPlay`
  (`parent.ReceiveBeginPlay`)
  (bind _asbp_hud (cast `/Game/Blueprints/HUD/BP_Hud` (`PlayerController.GetHUD` (`GameplayStatics.GetPlayerController` 0))))
  (`/Game/Blueprints/HUD/BP_Hud.showbphud` _asbp_hud)
  (bind _returnvalue (`|CreateWidget` "/Game/UI/W_PauseMenuBlueprint.W_PauseMenuBlueprint_C"))
  (bind _output_get (set `self.Pause Menu Widget` _returnvalue))
  (`Widget.SetVisibility` _output_get "Hidden")
  (`UserWidget.AddToViewport` _output_get 0))

(event `self.Health.Dead`
  (`KismetSystemLibrary.PrintString` "Estas Muerto Perro")
  (`GameplayStatics.OpenLevel` "Defeat"))

(event `self.Health.UpdateLifeEvent`
  (bind _health (`self.Health`))
  (bind _asbp_hud (cast `/Game/Blueprints/HUD/BP_Hud` (`PlayerController.GetHUD` (`GameplayStatics.GetPlayerController` 0))))
  (bind _hudreference (`/Game/Blueprints/HUD/BP_Hud.HudReference` _asbp_hud))
  (`/Engine/EditorBlueprintResources/StandardMacros.IsValid` _hudreference
    (:`Is Valid`
      (`/Game/UI/W_GameplayUIBlueprint.UpdateLife` _hudreference (`HealthComponent.CurrentHealth` _health) (`HealthComponent.MaxHealth` _health)))))

(event `EnhancedInput|/Game/ThirdPerson/Input/Actions/IA_Pause`
  (params (ActionValue :type Boolean) (ElapsedSeconds :type "Float (double-precision)") (TriggeredSeconds :type "Float (double-precision)") (InputAction :type "InputAction Object Reference" :default "/Game/ThirdPerson/Input/Actions/IA_Pause.IA_Pause"))
  (:`Triggered`
    (`GameplayStatics.SetGamePaused` true)
    (set `PlayerController.bShowMouseCursor` true (`GameplayStatics.GetPlayerController` 0))
    (`Widget.SetVisibility` (`self.Pause Menu Widget`) "Visible")))

(fn `GetAllGhostPoints`
  (returns (GhostPoints :type "Array of Vector Structure"))
  (bind _output_get (set `self.GhostPoints` (`|MakeArray` (`SceneComponent.K2_GetComponentLocation` (`self.GhostPoint4`)) (`SceneComponent.K2_GetComponentLocation` (`self.GhostPoint1`)) (`SceneComponent.K2_GetComponentLocation` (`self.GhostPoint2`)) (`SceneComponent.K2_GetComponentLocation` (`self.GhostPoint3`)))))
  (return _output_get))

(fn `UserConstructionScript`
  (`parent.UserConstructionScript`))