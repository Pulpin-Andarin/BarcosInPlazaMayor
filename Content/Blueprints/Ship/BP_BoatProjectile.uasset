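; Projectile fired by a gunner in ship combat, which damages boats and shows destruction effects on impact.
; Sphere overlaps with anything but the owning gunner hide the projectile mesh and trigger effects; boats also take damage once, with a sound played at world origin.
; Blocking hits on non-boat actors other than the gunner only hide it and trigger effects.
; Wood destruction and smoke particles are activated, then moved to the projectile's position.
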(event `self.ReceiveTick`
  (params (DeltaSeconds :type "Float (single-precision)")))

(event `self.SphereComponent.OnComponentBeginOverlap`
  (params (OverlappedComponent :type "PrimitiveComponent Object Reference") (OtherActor :type "Actor Object Reference") (OtherComp :type "PrimitiveComponent Object Reference") (OtherBodyIndex :type Integer) (bFromSweep :type Boolean) (SweepResult :type "HitResult Structure (by ref)"))
  (if (not (== OtherActor (`self.OwnerGunner`)))
    (`SceneComponent.SetVisibility` (`self.SphereProjectileComponent`) false false)
    (`self.Activate VFX`)
    (bind _asbp_boat (cast `/Game/Blueprints/Ship/BP_Boat` OtherActor))
    (`/Engine/EditorBlueprintResources/StandardMacros.DoOnce` false
      (:`Completed`
        (`HealthComponent.Damage` (`/Game/Blueprints/Ship/BP_Boat.Health` _asbp_boat) (`self.Damage`))
        (`GameplayStatics.PlaySoundAtLocation` "/Game/Sounds/TurboDamage.TurboDamage" (0.0 0.0 0.0) (struct) 1.0 1.0 0.0 null null null null)))))

(event `self.SphereProjectileComponent.OnComponentHit`
  (params (HitComponent :type "PrimitiveComponent Object Reference") (OtherActor :type "Actor Object Reference") (OtherComp :type "PrimitiveComponent Object Reference") (NormalImpulse :type "Vector Structure") (Hit :type "HitResult Structure (by ref)"))
  (if (not (== OtherActor (`self.OwnerGunner`)))
    (cast `/Game/Blueprints/Ship/BP_Boat` OtherActor
      (:`CastFailed`
        (`SceneComponent.SetVisibility` (`self.SphereProjectileComponent`) false false)
        (`self.Activate VFX`)))))

(fn `Activate Particle`
  (params (self2 :type "SceneComponent Object Reference"))
  (`ActorComponent.Activate` self2 false)
  (`SceneComponent.K2_SetWorldLocation` self2 (`SceneComponent.K2_GetComponentLocation` (`self.SphereProjectileComponent`)) false true))

(fn `Activate VFX`
  (`self.Activate Particle` (`self.P_WoodDestruction`))
  (`self.Activate Particle` (`self.P_Explosion_Smoke`)))

(fn `UserConstructionScript`)