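; Player boat Blueprint with charged left and right broadside shots and a timed rock wall ability (Muro).
; Holding a fire input runs a looping timer that raises launch impulse and redraws the predicted arc with spline meshes and an enemy-sensitive target decal.
; Release fires through BoatShootComponent and starts that side's reload, while component events toggle shot VFX.
; Space bar restores the zero-scaled rock and wall effect, then timers handle duration and cooldown.
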(event `self.ReceiveTick`
  (params (DeltaSeconds :type "Float (single-precision)")))

(event `EnhancedInput|/Game/ThirdPerson/Input/Actions/IA_ShootRight`
  (params (ActionValue :type Boolean) (ElapsedSeconds :type "Float (double-precision)") (TriggeredSeconds :type "Float (double-precision)") (InputAction :type "InputAction Object Reference" :default "/Game/ThirdPerson/Input/Actions/IA_ShootRight.IA_ShootRight"))
  (bind _boatshootcomponent (`self.BoatShootComponent`))
  (:`Started`
    (if (`BoatShootComponent.bReloadingRight` _boatshootcomponent)
      _
      (elif (not (`BoatShootComponent.bAiming` _boatshootcomponent))
        (bind _returnvalue (`KismetSystemLibrary.K2_SetTimerDelegate` (delegate `ShootRight`) 0.1 true))
        (set `self.RightTimerHandler` _returnvalue)
        (`self.InitValuesForPrediction`)
        (set `self.AimingRight` true))))
  (:`Completed`
    (if (`self.AimingRight`)
      (`BoatShootComponent.StartReloadingRightSide` (`self.BoatShootComponent`))
      (`self.ShootAndClearTimersInDirection` (`self.RightArrow`) (`self.RightTimerHandler`))
      (set `self.AimingRight` false))))

(event `ShootRight`
  (`self.ShowShootPrediction` (`self.RightArrow`)))

(event `EnhancedInput|/Game/ThirdPerson/Input/Actions/IA_ShootLeft`
  (params (ActionValue :type Boolean) (ElapsedSeconds :type "Float (double-precision)") (TriggeredSeconds :type "Float (double-precision)") (InputAction :type "InputAction Object Reference" :default "/Game/ThirdPerson/Input/Actions/IA_ShootLeft.IA_ShootLeft"))
  (:`Started`
    (if (`BoatShootComponent.bReloadingLeft` (`self.BoatShootComponent`))
      _
      (elif (not (`BoatShootComponent.bAiming` (`self.BoatShootComponent`)))
        (bind _returnvalue (`KismetSystemLibrary.K2_SetTimerDelegate` (delegate `ShootLeft`) 0.1 true))
        (set `self.LeftTimerHandler` _returnvalue)
        (`self.InitValuesForPrediction`)
        (set `self.AimingLeft` true))))
  (:`Completed`
    (if (`self.AimingLeft`)
      (`self.ShootAndClearTimersInDirection` (`self.LeftArrow`) (`self.LeftTimerHandler`))
      (set `self.AimingLeft` false)
      (`BoatShootComponent.StartReloadingLeftSide` (`self.BoatShootComponent`)))))

(event `ShootLeft`
  (`self.ShowShootPrediction` (`self.LeftArrow`)))

(event `self.BoatShootComponent.EndVfxRight`
  ;[1 1 1] VFX recharge
  (`ActorComponent.Deactivate` (`self.RightShoot`))
  (`ActorComponent.Deactivate` (`self.P_Explosion_right`)))

(event `self.BoatShootComponent.EndVfxLeft`
  ;[1 1 1] VFX recharge
  (`ActorComponent.Deactivate` (`self.LeftShoot`))
  (`ActorComponent.Deactivate` (`self.P_Explosion_Left`)))

(event `self.BoatShootComponent.StartVfxRight`
  ;[1 1 1] VFX recharge
  (`ActorComponent.Activate` (`self.RightShoot`) false)
  (`ActorComponent.Activate` (`self.P_Explosion_right`) false))

(event `self.BoatShootComponent.StartVfxLeft`
  ;[1 1 1] VFX recharge
  (`ActorComponent.Activate` (`self.LeftShoot`) false)
  (`ActorComponent.Activate` (`self.P_Explosion_Left`) false))

(event `self.ReceiveBeginPlay`
  (bind _rock (`self.ROCK`))
  (set `self.RockScale` (`SceneComponent.K2_GetComponentScale` _rock))
  (`SceneComponent.SetWorldScale3D` _rock (0.0 0.0 0.0))
  (`FXSystemComponent.SetFloatParameter` (`self.NS_Wall`) "DurationHability" (`self.HabilityDuration`))
  (`ActorComponent.SetActive` (`self.NS_Wall`) false false))

(event `Key|SpaceBar`
  (params (Key :type "Key Structure"))
  (bind _rock (`self.ROCK`))
  (:`Pressed`
    (if (`self.CanUseHability`)
      (set `self.IsHabilityActive` false)
      (`SceneComponent.SetHiddenInGame` _rock false false)
      (`SceneComponent.SetWorldScale3D` _rock (`self.RockScale`))
      (`ActorComponent.SetActive` (`self.NS_Wall`) true false)
      (set `self.CanUseHability` false)
      (`KismetSystemLibrary.K2_SetTimer` null "DisableHability" (`self.HabilityDuration`)))))

(fn `ActivateHability`
  (set `self.CanUseHability` true))

(fn `clear arc`
  (bind _spline_meshes (`self.Spline Meshes`))
  (`ActorComponent.K2_DestroyComponent` _spline_meshes)
  (`KismetArrayLibrary.Array_Clear` _spline_meshes)
  (`SplineComponent.ClearSplinePoints` (`self.Spline`) true))

(fn `DisableHability`
  (`SceneComponent.SetWorldScale3D` (`self.ROCK`) (0.0 0.0 0.0))
  (`ActorComponent.SetActive` (`self.NS_Wall`) false false)
  (`KismetSystemLibrary.K2_SetTimer` null "ActivateHability" (`self.CooldownHability`)))

(fn `InitValuesForPrediction`
  (bind _boatshootcomponent (`self.BoatShootComponent`))
  (`SceneComponent.SetVisibility` (`self.Sphere`) true false)
  (`SceneComponent.SetVisibility` (`self.DecalShootTarget`) true false)
  (set `BoatShootComponent.ActualImpulse` (`BoatShootComponent.MinImpulse` _boatshootcomponent) _boatshootcomponent)
  (set `BoatShootComponent.bAiming` true (`self.BoatShootComponent`)))

(fn `InitValuesForPrediction_0`
  (bind _boatshootcomponent (`self.BoatShootComponent`))
  (`SceneComponent.SetVisibility` (`self.DecalShootTarget`) true false)
  (set `BoatShootComponent.ActualImpulse` (`BoatShootComponent.MinImpulse` _boatshootcomponent) _boatshootcomponent)
  (set `BoatShootComponent.bAiming` true (`self.BoatShootComponent`)))

(fn `SetActualImpulse`
  (returns (ActualImpulse :type "Float (single-precision)"))
  (bind _boatshootcomponent (`self.BoatShootComponent`))
  (bind _actualimpulse (`BoatShootComponent.ActualImpulse` _boatshootcomponent))
  (set `BoatShootComponent.ActualImpulse` (`KismetMathLibrary.FClamp` (+ _actualimpulse (`BoatShootComponent.ImpulsIncrement` _boatshootcomponent)) (`BoatShootComponent.MinImpulse` _boatshootcomponent) (`BoatShootComponent.MaxImpulse` _boatshootcomponent)) _boatshootcomponent)
  (return _actualimpulse))

(fn `ShootAndClearTimersInDirection`
  (params (Arrow :type "ArrowComponent Object Reference") (TimerHandler :type "TimerHandle Structure"))
  (bind _boatshootcomponent (`self.BoatShootComponent`))
  (bind _boatshootcomponent_2 (`self.BoatShootComponent`))
  (`BoatShootComponent.Shoot` _boatshootcomponent (`KismetMathLibrary.MakeTransform` (`SceneComponent.K2_GetComponentLocation` Arrow) (`SceneComponent.K2_GetComponentRotation` Arrow)) (`BoatShootComponent.ActualImpulse` _boatshootcomponent))
  (`self.clear arc`)
  (`KismetSystemLibrary.K2_ClearAndInvalidateTimerHandle` TimerHandler)
  (`SceneComponent.SetVisibility` (`self.DecalShootTarget`) false false)
  (set `BoatShootComponent.ActualImpulse` (`BoatShootComponent.MinImpulse` _boatshootcomponent_2) _boatshootcomponent_2)
  (set `BoatShootComponent.bAiming` false (`self.BoatShootComponent`))
  (`SceneComponent.SetVisibility` (`self.Sphere`) false false))

(fn `ShowShootPrediction`
  (params (Arrow :type "ArrowComponent Object Reference"))
  (bind _decalshoottarget (`self.DecalShootTarget`))
  (bind _spline (`self.Spline`))
  (bind _spline_2 (`self.Spline`))
  (bind _actualimpulse (`self.SetActualImpulse`))
  (bind _output_get (set `self.LastLaunchVelocity` (* (`SceneComponent.GetForwardVector` Arrow) _actualimpulse)))
  (`self.clear arc`)
  (bind _predictresult (`GameplayStatics.Blueprint_PredictProjectilePath_Advanced` (make `PredictProjectilePathParams` :`StartLocation` (`SceneComponent.K2_GetComponentLocation` Arrow) :`LaunchVelocity` _output_get :`bTraceWithCollision` true :`ProjectileRadius` 5.0 :`MaxSimTime` 5.0 :`ActorsToIgnore` (`|MakeArray` self :!type "Actor Object Reference"))))
  (bind (_bblockinghit _binitialoverlap _time _distance _location _impactpoint _normal _impactnormal _physmat _hitactor) (`GameplayStatics.BreakHitResult` (`.HitResult` (break `PredictProjectilePathResult` _predictresult))))
  (bind _returnvalue (`KismetMathLibrary.Conv_VectorToRotator` _normal))
  (`SceneComponent.K2_SetWorldLocationAndRotation` (`self.Sphere`) _location _returnvalue false false)
  (cast `/Game/Blueprints/Enemies/BP_EnemyBase` _hitactor
    (:`then`
      (`DecalComponent.SetDecalMaterial` _decalshoottarget "/Game/Materials/M_ShootTargetFound.M_ShootTargetFound"))
    (:`CastFailed`
      (`DecalComponent.SetDecalMaterial` _decalshoottarget "/Game/Materials/M_ShootTargetr.M_ShootTargetr")))
  (`SceneComponent.K2_SetWorldLocationAndRotation` _decalshoottarget _location _returnvalue false false)
  (for _array_element (break `PredictProjectilePathResult` _predictresult)
    (`SplineComponent.AddSplinePoint` _spline (`.Location` (break `PredictProjectilePathPointData` _array_element)) "Local" true))
  (`SplineComponent.SetSplinePointType` _spline (`KismetArrayLibrary.Array_LastIndex` (break `PredictProjectilePathResult` _predictresult)) "CurveClamped" true)
  (for _index (range (`SplineComponent.GetNumberOfSplinePoints` (`self.Spline`)))
    (bind _returnvalue_2 (`AddComponent|NODE_AddSplineMeshComponent-1` :`bManualAttachment` true))
    (`KismetArrayLibrary.Array_Add` (`self.Spline Meshes`) _returnvalue_2)
    (bind (_location_2 _tangent) (`SplineComponent.GetLocationAndTangentAtSplinePoint` _spline_2 _index "Local"))
    (bind (_location_3 _tangent_2) (`SplineComponent.GetLocationAndTangentAtSplinePoint` _spline_2 (+ _index 1) "Local"))
    (`SplineMeshComponent.SetStartAndEnd` _returnvalue_2 _location_2 _tangent _location_3 _tangent_2 true)))

(fn `UserConstructionScript`)