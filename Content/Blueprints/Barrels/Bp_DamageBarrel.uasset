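; BP_DamageBarrel is an explosive barrel hazard that damages any BP_Boat overlapping its Root component.
; On overlap it spawns a large explosion particle, calls Damage on the boat's Health, and swaps the mesh to a transparent material to hide it.
; It destroys itself after a short delay, with nothing disabling overlaps during that wait.
; Debug prints and an impulse-like direction calculation are left unused.
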(event `self.Root.OnComponentBeginOverlap`
  (params (OverlappedComponent :type "PrimitiveComponent Object Reference") (OtherActor :type "Actor Object Reference") (OtherComp :type "PrimitiveComponent Object Reference") (OtherBodyIndex :type Integer) (bFromSweep :type Boolean) (SweepResult :type "HitResult Structure (by ref)"))
  (bind _asbp_boat (cast `/Game/Blueprints/Ship/BP_Boat` OtherActor))
  (`GameplayStatics.SpawnEmitterAtLocation` "/Game/Realistic_Starter_VFX_Pack_Vol2/Particles/Explosion/P_Explosion_Big_B.P_Explosion_Big_B" (`SceneComponent.K2_GetComponentLocation` (`self.Root`)) (struct) (2.0 2.0 2.0))
  (`PrimitiveComponent.SetMaterial` (`self.BarrelMesh`) 0 "/Game/Meshes/Boat/M_Transparent.M_Transparent")
  (`HealthComponent.Damage` (`/Game/Blueprints/Ship/BP_Boat.Health` _asbp_boat) 25)
  (`KismetSystemLibrary.Delay` 2.0)
  (`self.K2_DestroyActor`))

(event `self.ReceiveTick`
  (params (DeltaSeconds :type "Float (single-precision)")))

(fn `UserConstructionScript`)